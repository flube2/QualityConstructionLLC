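; A falling object hazard or platform that drops after the player character enters its box collider.
; If falling is allowed and physics is not yet active, it swaps to a warning material and plays a rumble.
; After a delay set by Difficulty, it plays a fall sound and enables physics simulation on the object.
; Both sounds play at the world origin rather than at the object.
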(event OnComponentBeginOverlap(BoxCollider)
  (params (OverlappedComponent :type Primitive%20Component%20Object%20Reference) (OtherActor :type Actor%20Object%20Reference) (OtherComp :type Primitive%20Component%20Object%20Reference) (OtherBodyIndex :type Integer) (bFromSweep :type Boolean) (SweepResult :type Hit%20Result%20Structure%20%28by%20ref%29))
  (if (== OtherActor (Game|GetPlayerCharacter 0))
    (CallFunction|Fall)))

(event Custom|Fall
  (if (Variables|Default|GetbCanFall)
    (if (not (Physics|IsSimulatingPhysics (Variables|Default|GetObject) "None"))
      (Rendering|Material|SetMaterial (Variables|Default|GetObject) 0 (Variables|Default|GetFallMaterial))
      (Audio|PlaySoundatLocation (Variables|Default|GetRumble) "0, 0, 0" "0, 0, 0" 1.0 1.0 0.0 0 0 0)
      (Utilities|FlowControl|Delay (Variables|Default|GetDifficulty))
      (Audio|PlaySoundatLocation (Variables|Default|GetFallSound) "0, 0, 0" "0, 0, 0" 1.0 1.0 0.0 0 0 0)
      (CallFunction|SimulatePhysics))))

(event EventBeginPlay)

(event EventTick
  (params (DeltaSeconds :type Float%20%28single-precision%29)))

(fn ConstructionScript)

(fn SimulatePhysics
  (Physics|SetSimulatePhysics (Variables|Default|GetObject) true))